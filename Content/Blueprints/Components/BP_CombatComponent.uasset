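; BP_CombatComponent is a component that tracks a main weapon and combat state.
; Setting a new weapon first calls OnUnequipped on any valid current weapon and destroys it, then stores the replacement.
; Changing the combat-enabled flag broadcasts OnCombatToggled with the new value.
; A reset function clears the attack count and saved-attack flag, and getters expose the weapon and combat state.
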(fn SetMainWeapon
  (params (NewWeapon :type BP%20Base%20Weapon%20Object%20Reference))
  ;[0.02416 0.02416 0.02416] Set Main Weapon
  (Utilities|FlowControl|Sequence
    (:then_0
      (Utilities|IsValid (Variables|Default|GetMainWeapon)
        (:Is%20Valid
          (Default|OnUnequipped (Variables|Default|GetMainWeapon))
          (Actor|DestroyActor (Variables|Default|GetMainWeapon)))))
    (:then_1
      (Variables|Default|SetMainWeapon NewWeapon))))

(fn GetMainWeapon
  ;[0.05127 0.05127 0.05127] Return main weapon
  (return (Variables|Default|GetMainWeapon)))

(fn SetCombatEnabled
  (params (bEnableCombat? :type Boolean))
  ;[0.02416 0.02416 0.02416] Set combat enabled
  (bind _output_get (Variables|Default|SetbCombatEnabled? bEnableCombat?))
  (Default|CallOnCombatToggled _output_get))

(fn IsCombatEnabled?
  ;[0.05127 0.05127 0.05127] Returns combat enabled
  (return (Variables|Default|GetbCombatEnabled?)))

(fn ResetAttack
  ;[0.05127 0.05127 0.05127] Reset attack count
  (Variables|Default|SetAttackCount 0)
  (Variables|Default|SetbIsAttackSaved? false))
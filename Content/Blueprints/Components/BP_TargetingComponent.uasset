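; Actor component that gives its owning character a toggleable lock-on to targets.
; A sphere trace along the follow camera's forward vector finds a Targeting_BPI actor, which is notified when targeting changes.
; While locked, Tick interpolates control rotation toward the target and releases it once it is untargetable or out of range.
; Toggling lock-on switches the character between camera-oriented and default rotation, based on combat state and movement speed mode.
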(event Custom|EnableLockOn
  ;[0.02416 0.02416 0.02416] Enable Lock On Logic
  (bind (_returnvalue _foundtarget) (CallFunction|FindTarget))
  (if (and _returnvalue (CallFunction|CanTargetActor? _foundtarget))
    (CallFunction|SetTargetActor _foundtarget)
    (CallFunction|SetIsTargeting true)
    (CallFunction|UpdateRotationMode)))

(event Custom|DisableLockOn
  ;[0.02416 0.02416 0.02416] Disable Lock On Logic
  (CallFunction|SetIsTargeting false)
  (CallFunction|SetTargetActor)
  (CallFunction|UpdateRotationMode))

(event Custom|ToggleLockOn
  ;[0.02416 0.02416 0.02416] Toggle on Lock On
  (if (not (CallFunction|GetIsTargeting))
    (CallFunction|EnableLockon)
    (else
      (CallFunction|DisableLockon))))

(event EventBeginPlay
  ;[0.02416 0.02416 0.02416] Get Starting Data
  (bind _ascharacter (Utilities|Casting|CastToCharacter (Components|GetOwner)))
  (Variables|Components|SetOwnerCharacter _ascharacter)
  (Variables|Components|SetOnwerController (Pawn|GetController (Variables|Components|GetOwnerCharacter)))
  (Variables|Default|SetFollowCam (Actor|GetComponentbyClass (Variables|Components|GetOwnerCharacter) "/Script/Engine.CameraComponent")))

(event EventTick
  (params (DeltaSeconds :type Float%20%28single-precision%29))
  ;[0.02416 0.02416 0.02416] Tick Event
  (if (Variables|Default|GetbIsTargeting?)
    (CallFunction|UpdateTargetingControlRotation)))

(fn SetIsTargeting
  (params (bIsTargeting? :type Boolean))
  (Variables|Default|SetbIsTargeting? bIsTargeting?)
  (bind _targetactor (Variables|Default|GetTargetActor)
    (:then
      (Class|TargetingBPI|OnTargeted(Message) _targetactor (Variables|Default|GetbIsTargeting?)))
    (:else)))

(fn GetIsTargeting
  (return (Variables|Default|GetbIsTargeting?)))

(fn FindTarget
  (bind (_outhit _returnvalue) (Collision|SphereTraceForObjects (Transformation|GetActorLocation (Components|GetOwner)) (+ (* (Math|Vector|GetForwardVector (Variables|Default|GetFollowCam)) (Variables|Initialization|GetTargetingDistance)) (Transformation|GetActorLocation (Components|GetOwner))) (Variables|Initialization|GetTargetingRadius) (Variables|Initialization|GetTargetObjectTypes) false (Utilities|Array|MakeArray (Components|GetOwner)) "None"))
  (if (and _returnvalue (Utilities|IsValid (.HitActor (Collision|BreakHitResult _outhit))))
    (if (Utilities|DoesObjectImplementInterface (.HitActor (Collision|BreakHitResult _outhit)) "/Game/Blueprints/Interfaces/Targeting_BPI.Targeting_BPI_C")
      (return true (.HitActor (Collision|BreakHitResult _outhit)))
      (else
        (return false 0)))
    (else
      (return false 0))))

(fn SetTargetActor
  (params (TargetActor :type Actor%20Object%20Reference))
  (Variables|Default|SetTargetActor TargetActor))

(fn GetTargetActor
  (return (Variables|Default|GetTargetActor)))

(fn UpdateTargetingControlRotation
  (bind _returnvalue (Utilities|Time|GetWorldDeltaSeconds))
  (bind _returnvalue_2 (Components|GetOwner))
  (bind _onwercontroller (Variables|Components|GetOnwerController))
  (bind _targetactor (Variables|Default|GetTargetActor))
  (bind _targetrotationinterpspeed (Variables|Initialization|GetTargetRotationInterpSpeed))
  (bind _returnvalue_3 (Transformation|GetActorRotation _onwercontroller))
  (bind _returnvalue_4 (Transformation|GetActorLocation _returnvalue_2))
  (bind _returnvalue_5 (Transformation|GetActorLocation _targetactor))
  (bind _returnvalue_6 (- _returnvalue_5 "0.000000,0.000000,100.000000"))
  (bind _returnvalue_7 (Math|Rotator|FindLookatRotation _returnvalue_4 _returnvalue_6))
  (bind _returnvalue_8 (Math|Interpolation|RInterpTo _returnvalue_3 _returnvalue_7 _returnvalue _targetrotationinterpspeed))
  ;[0.02416 0.02416 0.02416] Find Actual Rotation That Allows To Face Target Actor
  ;;[0.02416 0.02416 0.02416] Works Only if Data Is Valid
  (if (and (Utilities|IsValid (Variables|Components|GetOwnerCharacter)) (Utilities|IsValid (Variables|Default|GetTargetActor)))
    (if (CallFunction|CanTargetActor? (Variables|Default|GetTargetActor))
      (Pawn|SetControlRotation (Variables|Components|GetOnwerController) (Math|Rotator|MakeRotator (.Roll (Math|Rotator|BreakRotator _returnvalue_3)) (.pitch _returnvalue_8) (.yaw _returnvalue_8)))
      (else
        (CallFunction|DisableLockon)))))

(fn SetRotationMode
  (params (New%20Rotation%20Mode :type E_RotationMode%20Enum :default "NewEnumerator0"))
  (bind _ownercharacter (Variables|Components|GetOwnerCharacter))
  (bind _ownercharacter_2 (Variables|Components|GetOwnerCharacter))
  (bind _charactermovement (Variables|/Script/Engine.Character|GetCharacterMovement _ownercharacter))
  (bind _charactermovement_2 (Variables|/Script/Engine.Character|GetCharacterMovement _ownercharacter_2))
  (bind _output_get (Variables|Default|SetCurrentRotationMode New%20Rotation%20Mode))
  (switch Utilities|FlowControl|Switch|SwitchonE_RotationMode _output_get
    (:NewEnumerator0
      (Variables|/Script/Engine.Pawn|SetbUseControllerRotationYaw _ownercharacter_2 false)
      (Variables|/Script/Engine.CharacterMovementComponent|SetbUseControllerDesiredRotation _charactermovement_2 true)
      (Variables|/Script/Engine.CharacterMovementComponent|SetbOrientRotationToMovement _charactermovement_2 false))
    (:NewEnumerator1
      (Variables|/Script/Engine.Pawn|SetbUseControllerRotationYaw _ownercharacter false)
      (Variables|/Script/Engine.CharacterMovementComponent|SetbUseControllerDesiredRotation _charactermovement false)
      (Variables|/Script/Engine.CharacterMovementComponent|SetbOrientRotationToMovement _charactermovement true))))

(fn GetRotationMode
  (return (Variables|Default|GetCurrentRotationMode)))

(fn CanTargetActor?
  (params (InTargetActor :type Actor%20Object%20Reference))
  (Utilities|IsValid InTargetActor
    (:Is%20Valid
      (bind _returnvalue (Class|TargetingBPI|CanbeTargeted?(Message) InTargetActor))
      (return (and _returnvalue (< (Transformation|GetDistanceTo (Components|GetOwner) (Variables|Default|GetTargetActor)) (Variables|Initialization|GetTargetingDistance)))))
    (:Is%20Not%20Valid
      (return false))))

(fn UpdateRotationMode
  (Utilities|IsValid (Variables|Components|GetOwnerCombatComponent)
    (:Is%20Valid
      _)
    (:Is%20Not%20Valid
      (Variables|Components|SetOwnerCombatComponent (Actor|GetComponentbyClass (Variables|Components|GetOwnerCharacter) "/Game/Blueprints/Components/BP_CombatComponent.BP_CombatComponent_C"))))
  (bind _outvalue (Class|CombatBPI|GetMovementSpeedMode(Message) (Variables|Components|GetOwnerCharacter)))
  (CallFunction|SetRotationMode (select (Math|Boolean|ANDBoolean (Utilities|Enum|NotEqual(Enum) _outvalue "NewEnumerator2") (Default|IsCombatEnabled? (Variables|Components|GetOwnerCombatComponent)) (CallFunction|GetIsTargeting)) "NewEnumerator0" (Variables|Initialization|GetDefaultRotationMode))))
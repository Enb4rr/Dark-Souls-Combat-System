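; BP_CollisionComponent is an actor component that detects hits along a socket-to-socket segment on an assigned mesh, as used for melee-style hit windows.
; While collision is enabled, Tick runs a multi-sphere object trace between the start and end sockets.
; Each newly hit actor is recorded and broadcast once through OnHit, and enabling collision clears that record.
; Helper functions manage the ignore list and expose hit state.
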(event Custom|EnableCollision
  ;[0.05127 0.05127 0.05127] EnableCollision
  (CallFunction|ClearHitActors)
  (Variables|Default|SetbIsCollisionEnabled? true))

(event Custom|DisableCollision
  ;[0.05127 0.05127 0.05127] Disable Collisions
  (Variables|Default|SetbIsCollisionEnabled? false))

(event Custom|CollisionTrace
  (bind _collisionmeshcomponent (Variables|Default|GetCollisionMeshComponent))
  ;[0.05127 0.05127 0.05127] Collision Trace
  (bind _outhits (Collision|MultiSphereTraceForObjects (Transformation|GetSocketLocation _collisionmeshcomponent (Variables|Initialization|GetStartSocketName)) (Transformation|GetSocketLocation _collisionmeshcomponent (Variables|Initialization|GetEndSocketName)) (Variables|Initialization|GetTraceRadius) (Variables|Initialization|GetCollisionObjectTypes) false (Variables|Default|GetActorsToIgnore) (Variables|Initialization|GetDrawDebugType)))
  (for _array_element _outhits
    (bind _output_get (Variables|Default|SetLastHit _array_element))
    (if (not (Utilities|Array|ContainsItem (Variables|Default|GetAlreadyHitActors) (.HitActor (Collision|BreakHitResult _output_get))))
      (bind _output_get_2 (Variables|Default|SetHit%20Actor (.HitActor (Collision|BreakHitResult _output_get))))
      (Utilities|Array|Add (Variables|Default|GetAlreadyHitActors) _output_get_2)
      (Default|CallOnHit (Variables|Default|GetLastHit)))))

(event Custom|ClearHitActors
  ;[0.05127 0.05127 0.05127] Create Hit Actors
  (Utilities|Array|Clear (Variables|Default|GetAlreadyHitActors)))

(event Custom|SetCollisionMesh
  (params (MeshComponent :type Primitive%20Component%20Object%20Reference))
  ;[0.05127 0.05127 0.05127] Set Collision Mesh Component
  (Variables|Default|SetCollisionMeshComponent MeshComponent))

(event EventTick
  (params (DeltaSeconds :type Float%20%28single-precision%29))
  (if (Variables|Default|GetbIsCollisionEnabled?)
    (CallFunction|CollisionTrace)))

(fn GetAlreadyHitActors
  (return (Variables|Default|GetAlreadyHitActors)))

(fn IsCollisionEnabled?
  (return (Variables|Default|GetbIsCollisionEnabled?)))

(fn GetLastHit
  (return (Variables|Default|GetLastHit)))

(fn GetCollisionMesh
  (return (Variables|Default|GetCollisionMeshComponent)))

(fn AddActortoIgnore
  (params (InActor :type Actor%20Object%20Reference%20%28by%20ref%29))
  (Utilities|Array|AddUnique (Variables|Default|GetActorsToIgnore) InActor))

(fn RemoveActortoIgnore
  (params (InActor :type Actor%20Object%20Reference%20%28by%20ref%29))
  (Utilities|Array|RemoveItem (Variables|Default|GetActorsToIgnore) InActor))

(fn GetActorstoIgnore
  (return (Variables|Default|GetActorsToIgnore)))
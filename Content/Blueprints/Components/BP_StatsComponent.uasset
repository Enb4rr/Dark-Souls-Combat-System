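; Actor component that holds a character's stats, such as Health, Stamina and Armor, as base, max and current values.
; Current values initialize from base, and every write broadcasts an update, with modifications clamped between zero and max.
; Stamina regenerates on a looping timer after a retriggerable delay; other stats have no regen.
; TakeDamage scales damage against Armor, subtracts it from Health, and changes the owner's StateManager state at zero Health.
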(event Custom|StartRegen
  (params (StatType :type E_Stats%20Enum :default "NewEnumerator0"))
  (switch Utilities|FlowControl|Switch|SwitchonE_Stats StatType
    (:NewEnumerator2
      (Utilities|Time|ClearTimerbyFunctionName 0 "RegenStamina")
      (Utilities|FlowControl|RetriggerableDelay 1.2)
      (Utilities|Time|SetTimerbyFunctionName 0 "RegenStamina" 0.1 true))))

(fn SetCurrentStatValue
  (params (Stat :type E_Stats%20Enum :default "NewEnumerator0") (Value :type Float%20%28double-precision%29))
  (Utilities|Map|Add (Variables|CurrentStats|GetCurrent%20Stats) Stat Value)
  (Default|CallOnCurrentStatValueUpdated Stat Value))

(fn GetCurrentStatValue
  (params (Stat :type E_Stats%20Enum :default "NewEnumerator0"))
  (return (.Value (Utilities|Map|Find (Variables|CurrentStats|GetCurrent%20Stats) Stat))))

(fn InitializeStats
  (bind _keys (Utilities|Map|Keys (Variables|BaseStats|GetBase%20Stats)))
  (for _array_element _keys
    (CallFunction|SetCurrentStatValue _array_element (.basevalue (.Value (Utilities|Map|Find (Variables|BaseStats|GetBase%20Stats) _array_element))))))

(fn ModifyCurrentStatValue
  (params (Stat :type E_Stats%20Enum :default "NewEnumerator0") (Value :type Float%20%28double-precision%29) (ShouldRegen? :type Boolean))
  (if (!= Value 0.0)
    (bind _output_get (LocalVariables|SetL_Value (+ (CallFunction|GetCurrentStatValue Stat) Value)))
    (bind _output_get_2 (LocalVariables|SetL_Value (Math|Float|Clamp(Float) _output_get 0.0 (BaseStats|GetMaxStatValue Stat))))
    (CallFunction|SetCurrentStatValue Stat _output_get_2)
    (if ShouldRegen?
      (CallFunction|StartRegen Stat))))

(fn GetBaseStatValue
  (params (Stat :type E_Stats%20Enum :default "NewEnumerator0"))
  (return (.basevalue (.Value (Utilities|Map|Find (Variables|BaseStats|GetBase%20Stats) Stat)))))

(fn GetMaxStatValue
  (params (Stat :type E_Stats%20Enum :default "NewEnumerator0"))
  (return (.maxvalue (.Value (Utilities|Map|Find (Variables|BaseStats|GetBase%20Stats) Stat)))))

(fn SetBaseStatValue
  (params (Stat :type E_Stats%20Enum :default "NewEnumerator0") (Value :type Float%20%28double-precision%29))
  (bind _structout (Utilities|Struct|SetmembersinF_BaseStat (.Value (Utilities|Map|Find (Variables|BaseStats|GetBase%20Stats) Stat)) Value))
  (Utilities|Map|Add (Variables|BaseStats|GetBase%20Stats) Stat _structout))

(fn SetMaxStatValue
  (params (Stat :type E_Stats%20Enum :default "NewEnumerator0") (Value :type Float%20%28double-precision%29))
  (bind _structout (Utilities|Struct|SetmembersinF_BaseStat (.Value (Utilities|Map|Find (Variables|BaseStats|GetBase%20Stats) Stat)) Value))
  (Utilities|Map|Add (Variables|BaseStats|GetBase%20Stats) Stat _structout))

(fn TakeDamage
  (params (InDamage :type Float%20%28double-precision%29))
  (bind _value (CallFunction|GetCurrentStatValue "NewEnumerator3"))
  (bind _returnvalue (+ InDamage _value))
  (bind _returnvalue_2 (/ InDamage _returnvalue))
  (bind _returnvalue_3 (* InDamage _returnvalue_2))
  (LocalVariables|SetL_Damage (Math|Float|Clamp(Float) _returnvalue_3 0.0 _returnvalue_3))
  (CallFunction|ModifyCurrentStatValue "NewEnumerator1" (* (LocalVariables|GetL_Damage) -1.0) true)
  (Development|PrintString (Utilities|String|ToString(Float) (LocalVariables|GetL_Damage)))
  (if (<= (CallFunction|GetCurrentStatValue "NewEnumerator1") 0.0)
    (Default|SetState (Actor|GetComponentbyClass (Components|GetOwner) "/Game/Blueprints/Components/BP_StateManagerComponent.BP_StateManagerComponent_C") "NewEnumerator4")))

(fn RegenStamina
  (CallFunction|SetCurrentStatValue "NewEnumerator2" (Math|Float|Clamp(Float) (+ (CallFunction|GetCurrentStatValue "NewEnumerator2") (Variables|StatRegen|GetStaminaRegenRate)) 0.0 (BaseStats|GetMaxStatValue "NewEnumerator2")))
  (if (>= (CallFunction|GetCurrentStatValue "NewEnumerator2") (BaseStats|GetMaxStatValue "NewEnumerator2"))
    (Utilities|Time|ClearTimerbyFunctionName 0 "RegenStamina")))
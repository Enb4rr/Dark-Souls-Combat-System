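; Base dual-wield weapon actor that adds an off-hand mesh and right-foot strikes to its parent weapon.
; On equip and combat toggle, it snaps the off-hand mesh to a hand or stowed socket on the owning character.
; Collision components trace the off-hand and character meshes, ignore the owner, and switch on or off per collision part.
; Off-hand and foot hits apply point damage to actors that can receive it.
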(event OnHit(Off-HandWeaponCollisionComponent)
  (params (HitResult :type Hit%20Result%20Structure))
  (bind _hitactor (Collision|BreakHitResult HitResult))
  (bind _returnvalue (Class|CombatBPI|CanReceiveDamage(Message) _hitactor))
  (if _returnvalue
    (Game|Damage|ApplyPointDamage _hitactor (CallFunction|GetDamage) (Transformation|GetActorForwardVector (Components|GetOwner)) HitResult (Game|GetInstigatorController) self)))

(event OnHit(RightFootCollisionComponent)
  (params (HitResult :type Hit%20Result%20Structure))
  (bind _hitactor (Collision|BreakHitResult HitResult))
  (bind _returnvalue (Class|CombatBPI|CanReceiveDamage(Message) _hitactor))
  (if _returnvalue
    (Game|Damage|ApplyPointDamage _hitactor (CallFunction|GetDamage) (Transformation|GetActorForwardVector (Components|GetOwner)) HitResult (Game|GetInstigatorController) self)))

(event EventToggleCombat
  (params (bEnableCombat? :type Boolean))
  (|CallParentFunction bEnableCombat?)
  (CallFunction|AttachOff-HandWeapon (select bEnableCombat? (Variables|Initialization|GetSecond%20Weapon%20Hand%20Socket) (Variables|Initialization|GetSecond%20Weapon%20Attach%20Socket))))

(fn ConstructionScript
  (|CallParentFunction))

(fn ActivateCollision
  (params (Collision%20Part :type E_CollisionPart%20Enum :default "NewEnumerator0"))
  (switch Utilities|FlowControl|Switch|SwitchonE_CollisionPart Collision%20Part
    (:NewEnumerator0
      (Default|ActivateCollision (Variables|Default|GetMainWeaponCollisionComponent)))
    (:NewEnumerator1
      (Default|ActivateCollision (Variables|Default|GetOff-HandWeaponCollisionComponent)))
    (:NewEnumerator2
      (Default|ActivateCollision (Variables|Default|GetRightFootCollisionComponent)))))

(fn DeactivateCollision
  (params (Collision%20Part :type E_CollisionPart%20Enum :default "NewEnumerator0"))
  (switch Utilities|FlowControl|Switch|SwitchonE_CollisionPart Collision%20Part
    (:NewEnumerator0
      (Default|DeactivateCollision (Variables|Default|GetMainWeaponCollisionComponent)))
    (:NewEnumerator1
      (Default|DeactivateCollision (Variables|Default|GetOff-HandWeaponCollisionComponent)))
    (:NewEnumerator2
      (Default|DeactivateCollision (Variables|Default|GetRightFootCollisionComponent)))))

(fn OnEquipped
  (|CallParentFunction)
  (Default|SetCollisionMesh (Variables|Default|GetOff-HandWeaponCollisionComponent) (Variables|Default|GetOff-HandStaticMesh))
  (Default|SetCollisionMesh (Variables|Default|GetRightFootCollisionComponent) (Variables|/Script/Engine.Character|GetMesh (.AsCharacter (Utilities|Casting|CastToCharacter (Components|GetOwner)))))
  (CallFunction|AttachOff-HandWeapon (select (Default|IsCombatEnabled? (Variables|Default|GetCombatComponent)) (Variables|Initialization|GetSecond%20Weapon%20Hand%20Socket) (Variables|Initialization|GetSecond%20Weapon%20Attach%20Socket)))
  (Default|AddActortoIgnore (Variables|Default|GetOff-HandWeaponCollisionComponent) (Components|GetOwner))
  (Default|AddActortoIgnore (Variables|Default|GetRightFootCollisionComponent) (Components|GetOwner)))

(fn AttachOff-HandWeapon
  (params (Socket :type Name))
  (Transformation|AttachComponentToComponent (Variables|Default|GetOff-HandStaticMesh) (Variables|/Script/Engine.Character|GetMesh (.AsCharacter (Utilities|Casting|CastToCharacter (Components|GetOwner)))) Socket "SnapToTarget" "SnapToTarget" "SnapToTarget" true))
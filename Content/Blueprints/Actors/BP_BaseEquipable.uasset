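; BP_BaseEquipable is a base Blueprint for items a character can equip, tracking equipped state and providing shared mesh and attachment logic.
; OnEquipped sets the flag and calls AttachActor, which snaps the item to a socket on the owning Character's mesh.
; OnUnequipped only clears the flag, without detaching.
; GetItemMesh returns the static mesh component if its mesh is valid, otherwise the skeletal one.
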(fn ConstructionScript)

(fn GetItemMesh
  ;[0.05127 0.05127 0.05127] Return Item Mesh
  (Utilities|IsValid (Variables|/Script/Engine.StaticMeshComponent|GetStaticMesh (Variables|Default|GetItemStaticMesh))
    (:Is%20Valid
      (return (Variables|Default|GetItemStaticMesh)))
    (:Is%20Not%20Valid
      (return (Variables|Default|GetItemSkeletalMesh)))))

(fn OnEquipped
  ;[0.05127 0.05127 0.05127] On Equipped Base Func
  (Variables|Default|SetbIsEquipped? true)
  (ItemMesh|AttachActor (Variables|Initialization|GetAttach%20Socket%20Name)))

(fn OnUnequipped
  ;[0.05127 0.05127 0.05127] Unequipped Base Func
  (if (Variables|Default|GetbIsEquipped?)
    (Variables|Default|SetbIsEquipped? false)))

(fn AttachActor
  (params (SocketName :type Name))
  ;[0.05127 0.05127 0.05127] Attatch Actor Base Func
  (Transformation|AttachComponentToComponent (Variables|/Script/Engine.Character|GetMesh (.AsCharacter (Utilities|Casting|CastToCharacter (Components|GetOwner)))) SocketName "SnapToTarget" "SnapToTarget" "SnapToTarget" true))

(fn SetIsEquipped
  (params (isEquipped? :type Boolean))
  (Variables|Default|SetbIsEquipped? isEquipped?))

(fn IsEquipped?
  (return (Variables|Default|GetbIsEquipped?)))
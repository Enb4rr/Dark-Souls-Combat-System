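; BP_HumanoidEnemy is a humanoid enemy AI Blueprint that adds a health bar to its parent's behavior.
; On BeginPlay it creates a WB_HealthBar widget bound to its own StatsComponent, not the player's, and assigns it to the HealthBar widget component.
; The OnTargeted event shows or hides that bar as the enemy is targeted or untargeted, after calling the parent handler.
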(event EventBeginPlay
  (|CallParentFunction)
  (bind _returnvalue (UserInterface|CreateWidget "/Game/UI/WB_HealthBar.WB_HealthBar_C" (Game|GetPlayerController 0) (Variables|Default|GetStatsComponent) false))
  (UserInterface|SetWidget (Variables|Default|GetHealthBar) _returnvalue))

(event EventOnTargeted
  (params (bIsTargeted? :type Boolean))
  (|CallParentFunction bIsTargeted?)
  (Rendering|SetVisibility (Variables|Default|GetHealthBar) bIsTargeted? false))

(fn ConstructionScript
  (|CallParentFunction))
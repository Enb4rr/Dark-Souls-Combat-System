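; BP_MobEnemy is an enemy Blueprint that adds a physical weapon and a targeting health bar to its parent class.
; A stats-driven health bar widget is created on BeginPlay and shown only while the enemy is targeted.
; Weapon collision hits apply point damage from its stats to actors that can receive it.
; The weapon switches between hand and holster sockets when combat toggles, and simulates physics on death.
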(event OnHit(MainWeaponCollisionComponent)
  (params (HitResult :type Hit%20Result%20Structure))
  (bind _hitactor (Collision|BreakHitResult HitResult))
  (bind _returnvalue (Class|CombatBPI|CanReceiveDamage(Message) _hitactor))
  (if _returnvalue
    (Game|Damage|ApplyPointDamage _hitactor (Default|GetCurrentStatValue (Variables|Default|GetStatsComponent) "NewEnumerator4") (Transformation|GetActorForwardVector) HitResult (Pawn|GetController) self (Variables|Default|GetDamage%20Type%20Class))))

(event OnCombatToggled(CombatComponent)
  (params (bIsCombatEnabled? :type Boolean))
  (Transformation|AttachComponentToComponent (Variables|Default|GetWeaponMesh) (Variables|Character|GetMesh) (select bIsCombatEnabled? (Variables|Initialization|GetWeapon%20Hand%20Socket%20Name) (Variables|Initialization|GetAttach%20Socket%20Name)) "SnapToTarget" "SnapToTarget" "SnapToTarget" true))

(event Custom|SimulateWeaponPhysics
  (bind _weaponmesh (Variables|Default|GetWeaponMesh))
  (Collision|SetCollisionProfileName _weaponmesh "PhysicsActor" true :!class /Script/Engine.PrimitiveComponent)
  (Physics|SetSimulatePhysics _weaponmesh true))

(event EventBeginPlay
  (|CallParentFunction)
  (Default|SetCollisionMesh (Variables|Default|GetMainWeaponCollisionComponent) (Variables|Default|GetWeaponMesh))
  (bind _returnvalue (UserInterface|CreateWidget "/Game/UI/WB_HealthBar.WB_HealthBar_C" (Game|GetPlayerController 0) (Variables|Default|GetStatsComponent) false))
  (UserInterface|SetWidget (Variables|Default|GetHealthBar) _returnvalue))

(event EventPerformDeath
  (|CallParentFunction)
  (CallFunction|SimulateWeaponPhysics))

(event EventOnTargeted
  (params (bIsTargeted? :type Boolean))
  (|CallParentFunction bIsTargeted?)
  (Rendering|SetVisibility (Variables|Default|GetHealthBar) bIsTargeted? false))

(fn ConstructionScript
  (|CallParentFunction))
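; Test dummy character that can be locked on to and damaged, reacting to hits.
; On BeginPlay it initializes its stats component and spawns and equips its starting equipment.
; Point damage feeds the stats component and plays impact sound and blood, then, if a hit reaction is allowed, sets the Disabled state tag and plays a react montage.
; Targeting toggles the lock-on widget and is refused while the state manager reports Dead.
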(event EventBeginPlay
  (bind _self self)
  (Default|InitializeStats (Variables|Default|GetStatsComponent))
  (for _array_element (Variables|Default|GetStartingEquipment)
    (bind _returnvalue (Game|SpawnActorfromClass _array_element (Transformation|GetActorTransform) "Undefined" "MultiplyWithRoot" _self _self))
    (Default|OnEquipped _returnvalue)))

(event EventOnTargeted
  (params (bIsTargeted? :type Boolean))
  (Rendering|SetVisibility (Variables|Default|GetLockOnWidget) bIsTargeted? false))

(event Game|Damage|EventPointDamage
  (params (Damage :type Float%20%28single-precision%29) (DamageType :type Damage%20Type%20Object%20Reference) (HitLocation :type Vector :default "0, 0, 0") (HitNormal :type Vector :default "0, 0, 0") (HitComponent :type Primitive%20Component%20Object%20Reference) (BoneName :type Name :default "None") (ShotFromDirection :type Vector :default "0, 0, 0") (InstigatedBy :type Controller%20Object%20Reference) (DamageCauser :type Actor%20Object%20Reference) (HitInfo :type Hit%20Result%20Structure%20%28by%20ref%29))
  (Default|TakeDamage (Variables|Default|GetStatsComponent) Damage)
  (Audio|PlaySoundatLocation "/Game/Assets/SoundFX/Gruntling/A_Guardian_Impact_Cue.A_Guardian_Impact_Cue" HitLocation "0, 0, 0" 1.0 1.0 0.0 0 0 0 0)
  (Effects|SpawnEmitteratLocation "/Game/VFX/Particles/Blood/P_Blood_Splat_Cone.P_Blood_Splat_Cone" HitLocation)
  (if (CallFunction|CanReceiveHitReaction?)
    (Default|SetState (Variables|Default|GetStateManagerComponent) "(TagName=\"Character.State.Disabled\")")
    (Animation|PlayAnimMontage "/Game/Assets/Animations/HitReactions/Standing_React_Large_Front_Montage.Standing_React_Large_Front_Montage" 1.0 "None")))

(fn ConstructionScript
  (|CallParentFunction))

(fn CanbeTargeted?
  (return (not (Default|IsCurrentStateEqualtoAny? (Variables|Default|GetStateManagerComponent) "(GameplayTags=((TagName=\"Character.State.Dead\")))"))))
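; Base weapon actor for the combat system that equips onto a character and deals damage on hits.
; On equip it attaches to the hand or holster socket based on combat state, registers as main weapon, and updates the animation combat type.
; Its collision component traces against the item mesh, ignoring the owner, and hits apply point damage to actors that accept it.
; A separate event switches the mesh to simulated physics.
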(event OnHit(BP_CollisionComponent)
  (params (HitResult :type Hit%20Result%20Structure))
  (bind _hitactor (Collision|BreakHitResult HitResult))
  ;[0.05127 0.05127 0.05127] Manage hit detection
  (bind _returnvalue (Class|CombatBPI|CanReceiveDamage(Message) _hitactor))
  (if _returnvalue
    (Game|Damage|ApplyPointDamage _hitactor (Variables|Default|GetDamage) (Transformation|GetActorForwardVector (Components|GetOwner)) HitResult (Game|GetInstigatorController) self)))

(event Custom|SimulateWeaponPhysics
  (bind _returnvalue (CallFunction|GetItemMesh))
  (Collision|SetCollisionProfileName _returnvalue "PhysicsActor" true :!class /Script/Engine.PrimitiveComponent)
  (Physics|SetSimulatePhysics _returnvalue true))

(fn ConstructionScript
  (|CallParentFunction))

(fn OnEquipped
  ;[0.05127 0.05127 0.05127] On Equipped Weapon Functionality
  (Variables|Default|SetCombatComponent (Actor|GetComponentbyClass (Components|GetOwner) "/Game/CombatSystem/Blueprints/Components/BP_CombatComponent.BP_CombatComponent_C"))
  (CallFunction|AttachActor (select (Default|IsCombatEnabled? (Variables|Default|GetCombatComponent)) (Variables|Initialization|GetHandSocketName) (Variables|Default|GetAttach%20Socket%20Name)))
  (Default|SetMainWeapon (Variables|Default|GetCombatComponent) self)
  (Class|AnimInstaceBPI|UpdateCombatType(Message) (Components|SkeletalMesh|GetAnimInstance (Variables|/Script/Engine.Character|GetMesh (.AsCharacter (Utilities|Casting|CastToCharacter (Components|GetOwner))))) (Variables|Initialization|GetCombatType))
  (Default|SetCollisionMesh (Variables|Default|GetBP_CollisionComponent) (CallFunction|GetItemMesh))
  (Default|AddActortoIgnore (Variables|Default|GetBP_CollisionComponent) (Components|GetOwner)))